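; Dodge roll ability that runs a dodge roll special move on the owning character when activated.
; Activation requires non-zero desired movement input from the TPP player controller and a character that is not falling.
; It is also blocked while the movement component reports that the character wants to slide but has not yet started the slide.
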(event `self.OnAbilityActivated`
  (`TPPPlayerCharacter.ExecuteSpecialMoveByClass` (`self.OwningCharacter`) (`self.DodgeRollClass`)))

(fn `CanActivate`
  (returns (ReturnValue :type Boolean))
  (bind _owningcharacter (`self.OwningCharacter`))
  (bind _returnvalue (`TPPPlayerCharacter.GetTPPMovementComponent` _owningcharacter))
  (bind _returnvalue_2 (`TPPMovementComponent.DoesCharacterWantToSlide` _returnvalue))
  (return (and (not (`KismetMathLibrary.Vector_IsZero` (`TPPPlayerController.GetDesiredMovementDirection` (`TPPPlayerCharacter.GetTPPPlayerController` _owningcharacter)))) (not (`NavMovementComponent.IsFalling` (`Character.CharacterMovement` _owningcharacter))) (or (not _returnvalue_2) (and _returnvalue_2 (`TPPMovementComponent.HasCharacterStartedSlide` _returnvalue))))))