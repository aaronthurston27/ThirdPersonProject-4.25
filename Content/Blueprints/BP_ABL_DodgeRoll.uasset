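; BP_ABL_DodgeRoll is an ability that makes the owning character perform a dodge roll.
; On activation it passes DodgeRollClass to the character's ExecuteSpecialMove, so the roll itself lives in that special move.
; CanActivate allows it only while the third-person player controller reports a non-zero desired movement direction and the character is not falling.
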(event `self.OnAbilityActivated`
  (`ThirdPersonProjectCharacter.ExecuteSpecialMove` (`self.OwningCharacter`) (`self.DodgeRollClass`)))

(fn `CanActivate`
  (returns (ReturnValue :type Boolean))
  (bind _owningcharacter (`self.OwningCharacter`))
  (return (and (not (`KismetMathLibrary.Vector_IsZero` (`TPPPlayerController.GetDesiredMovementDirection` (`ThirdPersonProjectCharacter.GetTPPPlayerController` _owningcharacter)))) (not (`NavMovementComponent.IsFalling` (`Character.CharacterMovement` _owningcharacter))))))