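; Weapon ammo pickup that refills the reserve pool of the collecting character's currently equipped weapon.
; CanPickup passes only when that weapon is valid, uses the pickup's ammo type and has room left in its pool.
; ObtainPickup adds the pickup amount, capped at the remaining pool space and leaving chambered ammo untouched, then calls the parent pickup logic.
; Overlap events only print a debug string.
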(event `self.ObtainPickup`
  (params (InstigatorCharacter :type "TPPPlayerCharacter Object Reference"))
  (`self.AddAmmoToCharacter` InstigatorCharacter)
  (`parent.ObtainPickup` InstigatorCharacter))

(event `self.ReceiveActorBeginOverlap`
  (params (OtherActor :type "Actor Object Reference"))
  (`KismetSystemLibrary.PrintString` "Hello" :!label _label))

(event `self.StaticMesh.OnComponentBeginOverlap`
  (params (OverlappedComponent :type "PrimitiveComponent Object Reference") (OtherActor :type "Actor Object Reference") (OtherComp :type "PrimitiveComponent Object Reference") (OtherBodyIndex :type Integer) (bFromSweep :type Boolean) (SweepResult :type "HitResult Structure (by ref)"))
  (goto _label))

(fn `AddAmmoToCharacter`
  (params (TargetCharacter :type "TPPPlayerCharacter Object Reference"))
  (bind _returnvalue (`TPPPlayerCharacter.GetCurrentEquippedWeapon` TargetCharacter))
  (if (`KismetSystemLibrary.IsValid` TargetCharacter)
    (if (`KismetSystemLibrary.IsValid` _returnvalue)
      (`TPPWeaponBase.ModifyWeaponAmmo` _returnvalue 0 (`KismetMathLibrary.Min` (`self.AmmoPickupAmount`) (- (`TPPWeaponBase.MaxAmmoInPool` _returnvalue) (`TPPWeaponBase.GetCurrentPooledAmmo` _returnvalue)))))))

(fn `CanPickup`
  (params (CharacterInstigator :type "TPPPlayerCharacter Object Reference"))
  (returns (ReturnValue :type Boolean))
  (bind _returnvalue (`TPPPlayerCharacter.GetCurrentEquippedWeapon` CharacterInstigator))
  (if (`KismetSystemLibrary.IsValid` CharacterInstigator)
    (if (`KismetSystemLibrary.IsValid` _returnvalue)
      (return (and (`|EnumEquality` (`self.PickupAmmoType`) (`TPPWeaponBase.AmmoType` _returnvalue)) (< (`TPPWeaponBase.GetCurrentPooledAmmo` _returnvalue) (`TPPWeaponBase.MaxAmmoInPool` _returnvalue))))
      (else
        _)))
  (return false))

(fn `UserConstructionScript`)